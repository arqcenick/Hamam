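; An inspectable scrubber item that the player rubs on customers (BP_Musteri) by moving the mouse over their belly.
; InspectMesh overlaps with "Belly"-tagged actors set Entered on the scrubber.
; Each tick, mouse travel feeds the Accumulator of customers also flagged Entered, while every customer's value steadily decays within a clamped range.
; StartInspection disables physics, attaches the scrubber to the player's Item and moves it in front of the camera.
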(event OnComponentBeginOverlap(InspectMesh)
  (params (OverlappedComponent :type Primitive%20Component%20Object%20Reference) (OtherActor :type Actor%20Object%20Reference) (OtherComp :type Primitive%20Component%20Object%20Reference) (OtherBodyIndex :type Integer) (bFromSweep :type Boolean) (SweepResult :type Hit%20Result%20Structure%20%28by%20ref%29))
  (if (Utilities|Array|ContainsItem (Variables|/Script/Engine.Actor|GetTags OtherActor) "Belly")
    (if (not (Variables|Default|GetEntered))
      (Variables|Default|SetEntered true))))

(event OnComponentEndOverlap(InspectMesh)
  (params (OverlappedComponent :type Primitive%20Component%20Object%20Reference) (OtherActor :type Actor%20Object%20Reference) (OtherComp :type Primitive%20Component%20Object%20Reference) (OtherBodyIndex :type Integer))
  (if (Utilities|Array|ContainsItem (Variables|/Script/Engine.Actor|GetTags OtherActor) "Belly")
    (if (Variables|Default|GetEntered)
      (Variables|Default|SetEntered false))))

(event EventTick
  (params (DeltaSeconds :type Float%20%28single-precision%29))
  (|CallParentFunction DeltaSeconds)
  (bind _returnvalue (Class|WidgetLayoutLibrary|GetMousePositiononViewport))
  (bind _outactors (Actor|GetAllActorsOfClass "/Game/DoomsDayge/Blueprints/BP_Musteri.BP_Musteri_C"))
  (for _array_element _outactors
    (if (and (Variables|/Game/DoomsDayge/Blueprints/BP_Musteri.BP_Musteri_C|GetEntered _array_element) (Variables|Default|GetEntered))
      (Variables|/Game/DoomsDayge/Blueprints/BP_Musteri.BP_Musteri_C|SetAccumulator _array_element (+ (/ (* (Math|Vector2D|Vector2DLength (- _returnvalue (Variables|Default|GetLastMousePos))) (Utilities|Time|GetWorldDeltaSeconds)) 0.2) (Variables|/Game/DoomsDayge/Blueprints/BP_Musteri.BP_Musteri_C|GetAccumulator _array_element))))
    (Variables|/Game/DoomsDayge/Blueprints/BP_Musteri.BP_Musteri_C|SetAccumulator _array_element (Math|Float|Clamp(Float) (- (Variables|/Game/DoomsDayge/Blueprints/BP_Musteri.BP_Musteri_C|GetAccumulator _array_element) (* (Utilities|Time|GetWorldDeltaSeconds) 2e+01)) 0.0 4e+02)))
  (Variables|Default|SetLastMousePos _returnvalue))

(fn ConstructionScript
  (|CallParentFunction))

(fn StartInspection
  (bind _returnvalue (Game|GetPlayerCameraManager 0))
  (bind _inspectmesh (Variables|Default|GetInspectMesh))
  (Input|EnableInput (Game|GetPlayerController 0))
  (Physics|SetSimulatePhysics _inspectmesh false)
  (Collision|SetCollisionEnabled _inspectmesh "QueryOnly")
  (Transformation|AttachComponentToComponent (Variables|/Game/FirstPerson/Blueprints/BP_FirstPersonCharacter.BP_FirstPersonCharacter_C|GetItem (Variables|Default|GetPlayer%20Character)) "None" "KeepRelative" "KeepRelative" "KeepRelative" false)
  (Variables|/Game/FirstPerson/Blueprints/BP_FirstPersonCharacter.BP_FirstPersonCharacter_C|SetCurrentItem (Variables|Default|GetPlayer%20Character) self)
  (Transformation|SetActorLocation (+ (Camera|GetCameraLocation _returnvalue) (* (Math|Vector|GetForwardVector (Camera|GetCameraRotation _returnvalue)) (Variables|Default|GetInspectDistance))) false false))