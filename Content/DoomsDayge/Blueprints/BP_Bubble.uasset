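; BP_Bubble is a short-lived bubble actor that fades out and destroys itself.
; BeginPlay creates a dynamic material instance on its static mesh and picks a random lifetime of a few seconds.
; Tick counts the remaining time down, remaps it to the material's Transparency parameter, and destroys the actor when that value nears zero.
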(event EventTick
  (params (DeltaSeconds :type Float%20%28single-precision%29))
  (Variables|Default|SetRemainingTime (- (Variables|Default|GetRemainingTime) (* DeltaSeconds 1.0)))
  (Rendering|Material|SetScalarParameterValue (Variables|Default|GetNewVar) "Transparency" (Math|Float|MapRangeClamped (- (Variables|Default|GetRemainingTime) (* DeltaSeconds 1.0)) (Variables|Default|GetMaxTime) 0.0 1.0 0.0) :!class /Script/Engine.MaterialInstanceDynamic)
  (if (< (Math|Float|MapRangeClamped (- (Variables|Default|GetRemainingTime) (* DeltaSeconds 1.0)) (Variables|Default|GetMaxTime) 0.0 1.0 0.0) 0.05)
    (Actor|DestroyActor)))

(event EventBeginPlay
  (bind _returnvalue (Rendering|Material|CreateDynamicMaterialInstance (Variables|Default|GetStaticMesh) 0 (Rendering|Material|GetMaterial (Variables|Default|GetStaticMesh) 0) "None" :!class /Script/Engine.PrimitiveComponent))
  (Variables|Default|SetNewVar _returnvalue)
  (bind _output_get (Variables|Default|SetRemainingTime (Math|Random|RandomFloatinRange 1.0 3.0)))
  (Variables|Default|SetMaxTime _output_get))

(fn ConstructionScript)