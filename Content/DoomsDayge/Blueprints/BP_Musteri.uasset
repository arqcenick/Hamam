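; Customer (Musteri) actor that the player can pick up, carry and drop as a ragdoll, with a look-at prompt.
; Interact attaches it in front of the camera or detaches it with physics re-enabled.
; Adding a pestemal tints its last material red and enables interaction after a delay.
; When dirty and its externally fed Accumulator passes a random threshold, it stands up, plays a completion sound and increments the player's satisfied-customer count.
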(event OnComponentBeginOverlap(SkeletalMesh)
  (params (OverlappedComponent :type Primitive%20Component%20Object%20Reference) (OtherActor :type Actor%20Object%20Reference) (OtherComp :type Primitive%20Component%20Object%20Reference) (OtherBodyIndex :type Integer) (bFromSweep :type Boolean) (SweepResult :type Hit%20Result%20Structure%20%28by%20ref%29))
  (if (Utilities|Array|ContainsItem (Variables|/Script/Engine.Actor|GetTags OtherActor) "Belly")
    (if (not (Variables|Default|GetEntered))
      (Variables|Default|SetEntered true))))

(event OnComponentEndOverlap(SkeletalMesh)
  (params (OverlappedComponent :type Primitive%20Component%20Object%20Reference) (OtherActor :type Actor%20Object%20Reference) (OtherComp :type Primitive%20Component%20Object%20Reference) (OtherBodyIndex :type Integer))
  (if (Utilities|Array|ContainsItem (Variables|/Script/Engine.Actor|GetTags OtherActor) "Belly")
    (if (Variables|Default|GetEntered)
      (Variables|Default|SetEntered false))))

(event Custom|GettingUp
  (params (isDirty :type Boolean%20%28by%20ref%29))
  (bind _skeletalmesh (Variables|Default|GetSkeletalMesh))
  (bind _returnvalue (Transformation|GetBoneTransform _skeletalmesh "Hips" "RTS_World"))
  (if isDirty
    (if (> (Variables|Default|GetAccumulator) (Variables|Default|GetAccumulatorMax))
      (Transformation|SetRelativeLocation (Variables|Default|GetSkeletalMesh) (Math|Vector|MakeVector (.x (.location _returnvalue)) (.y (.location _returnvalue)) 63.915585) false false)
      (Physics|SetSimulatePhysics (Variables|Default|GetSkeletalMesh) false)
      (Transformation|SetWorldRotation (Variables|Default|GetSkeletalMesh) (Math|Rotator|MakeRotator 0.0 0.0 1.8e+02) false true)
      (Variables|Default|SetIs%20Dirty false)
      (Variables|Default|SetInteractable false)
      (Components|Animation|PlayAnimation (Variables|Default|GetSkeletalMesh) (Variables|Default|GetStandUpAnimation) false)
      (bind _returnvalue_2 (Actor|GetActorOfClass "/Game/Sound/BP_SoundController.BP_SoundController_C"))
      (Default|PlayCompletionSound _returnvalue_2)
      (bind _returnvalue_3 (Actor|GetActorOfClass "/Game/FirstPerson/Blueprints/BP_FirstPersonCharacter.BP_FirstPersonCharacter_C"))
      (Variables|/Game/FirstPerson/Blueprints/BP_FirstPersonCharacter.BP_FirstPersonCharacter_C|SetMusterisSatisfied _returnvalue_3 (+ (Variables|/Game/FirstPerson/Blueprints/BP_FirstPersonCharacter.BP_FirstPersonCharacter_C|GetMusterisSatisfied _returnvalue_3) 1)))))

(event Custom|OnPestemalAdded
  (bind _skeletalmesh (Variables|Default|GetSkeletalMesh))
  (bind _returnvalue (Rendering|Material|GetNumMaterials _skeletalmesh))
  (bind _returnvalue_2 (- _returnvalue 1))
  ;[0.15 0.15 0.15 0.5] Comment
  (bind _returnvalue_3 (Rendering|Material|CreateDynamicMaterialInstance (Variables|Default|GetSkeletalMesh) _returnvalue_2 (Rendering|Material|GetMaterial _skeletalmesh _returnvalue_2) "None" :!class /Script/Engine.PrimitiveComponent))
  (Rendering|Material|SetMaterial (Variables|Default|GetSkeletalMesh) _returnvalue_2 _returnvalue_3)
  (Rendering|Material|SetVectorParameterValue _returnvalue_3 "Color" "(R=1.000000,G=0.000000,B=0.000000,A=1.000000)" :!class /Script/Engine.MaterialInstanceDynamic)
  (Utilities|FlowControl|Delay 5.0)
  (Variables|Default|SetInteractable true))

(event Custom|dropkeysound)

(event EventBeginPlay
  (Variables|Default|SetAccumulatorMax (Math|Random|RandomFloatinRange 1e+02 3e+02)))

(event EventInteractwith
  (params (PlayerCharacter :type BP%20First%20Person%20Character%20Object%20Reference))
  (bind _output_get (Variables|Default|SetPlayer%20Character PlayerCharacter))
  (bind _musteriitem (Variables|/Game/FirstPerson/Blueprints/BP_FirstPersonCharacter.BP_FirstPersonCharacter_C|GetMusteriItem _output_get)
    (:then
      (CallFunction|StopInspection _musteriitem)
      (Variables|/Game/FirstPerson/Blueprints/BP_FirstPersonCharacter.BP_FirstPersonCharacter_C|SetMusteriItem _output_get 0)
      (Variables|/Game/FirstPerson/Blueprints/BP_FirstPersonCharacter.BP_FirstPersonCharacter_C|SetIsGrabbed _output_get false))
    (:else
      (if (Variables|Default|GetInteractable)
        (CallFunction|StartInspection)
        (Variables|/Game/FirstPerson/Blueprints/BP_FirstPersonCharacter.BP_FirstPersonCharacter_C|SetIsGrabbed (Variables|Default|GetPlayer%20Character) true)
        (Rendering|SetVisibility (Variables|Default|GetE_Prompt_Widget) false false)))))

(event EventTick
  (params (DeltaSeconds :type Float%20%28single-precision%29))
  (Utilities|FlowControl|Sequence
    (:then_0
      (CallFunction|GettingUp (Variables|Default|GetIs%20Dirty)))
    (:then_1
      (bind _asbp_first_person_character (Utilities|Casting|CastToBP_FirstPersonCharacter (Game|Player|GetPlayerPawn 0)))
      (if (not (Variables|/Game/FirstPerson/Blueprints/BP_FirstPersonCharacter.BP_FirstPersonCharacter_C|GetIsGrabbed _asbp_first_person_character))
        (if (== self (Variables|/Game/FirstPerson/Blueprints/BP_FirstPersonCharacter.BP_FirstPersonCharacter_C|GetLookAtActor _asbp_first_person_character))
          (Rendering|SetVisibility (Variables|Default|GetE_Prompt_Widget) true false)
          (else
            (Rendering|SetVisibility (Variables|Default|GetE_Prompt_Widget) false false)))))))

(fn ConstructionScript)

(fn StartInspection
  (bind _returnvalue (Game|GetPlayerCameraManager 0))
  (Input|EnableInput (Game|GetPlayerController 0))
  (Collision|SetCollisionEnabled (Variables|Default|GetSkeletalMesh) "NoCollision")
  (Transformation|AttachComponentToComponent (Variables|/Game/FirstPerson/Blueprints/BP_FirstPersonCharacter.BP_FirstPersonCharacter_C|GetItem (Variables|Default|GetPlayer%20Character)) "None" "KeepWorld" "KeepRelative" "KeepRelative" false)
  (Collision|SetCollisionEnabled (Variables|Default|GetSkeletalMesh) "NoCollision")
  (Variables|/Game/FirstPerson/Blueprints/BP_FirstPersonCharacter.BP_FirstPersonCharacter_C|SetMusteriItem (Variables|Default|GetPlayer%20Character) self)
  (Transformation|SetActorLocation (+ (* (Math|Vector|GetForwardVector (Camera|GetCameraRotation _returnvalue)) (Variables|Default|GetInspectDistance)) (Camera|GetCameraLocation _returnvalue)) false false))

(fn StopInspection
  (Transformation|DetachFromActor "KeepWorld" "KeepWorld" "KeepWorld")
  (Physics|SetSimulatePhysics (Variables|Default|GetSkeletalMesh) true)
  (Collision|SetCollisionEnabled (Variables|Default|GetSkeletalMesh) "QueryAndPhysics"))