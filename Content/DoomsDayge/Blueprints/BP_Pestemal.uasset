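; BP_Pestemal is a pestemal pickup that is handed to a customer (BP_Musteri) when its InspectMesh overlaps an actor tagged "Belly".
; An Entered flag guards repeat overlaps and resets on end overlap.
; It updates only the first customer found in the level, setting HasPestemal true if that customer has entered and is not dirty.
; It then calls OnPestemalAdded regardless of that result and destroys itself.
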(event OnComponentBeginOverlap(InspectMesh)
  (params (OverlappedComponent :type Primitive%20Component%20Object%20Reference) (OtherActor :type Actor%20Object%20Reference) (OtherComp :type Primitive%20Component%20Object%20Reference) (OtherBodyIndex :type Integer) (bFromSweep :type Boolean) (SweepResult :type Hit%20Result%20Structure%20%28by%20ref%29))
  (if (Utilities|Array|ContainsItem (Variables|/Script/Engine.Actor|GetTags OtherActor) "Belly")
    (if (not (Variables|Default|GetEntered))
      (Variables|Default|SetEntered true)
      (bind _outactors (Actor|GetAllActorsOfClass "/Game/DoomsDayge/Blueprints/BP_Musteri.BP_Musteri_C"))
      (bind _array_element (Utilities|Array|ForEachLoopwithBreak _outactors :!label _label)
        (:LoopBody
          (Variables|/Game/DoomsDayge/Blueprints/BP_Musteri.BP_Musteri_C|SetHasPestemal _array_element (and (not (Variables|/Game/DoomsDayge/Blueprints/BP_Musteri.BP_Musteri_C|GetIs%20Dirty _array_element)) (Variables|/Game/DoomsDayge/Blueprints/BP_Musteri.BP_Musteri_C|GetEntered _array_element)))
          (Default|OnPestemalAdded _array_element)
          (Variables|Default|SetWillBeDestroyed true)
          (goto _label Break))
        (:Completed
          (if (Variables|Default|GetWillBeDestroyed)
            (Actor|DestroyActor)))))))

(event OnComponentEndOverlap(InspectMesh)
  (params (OverlappedComponent :type Primitive%20Component%20Object%20Reference) (OtherActor :type Actor%20Object%20Reference) (OtherComp :type Primitive%20Component%20Object%20Reference) (OtherBodyIndex :type Integer))
  (if (Utilities|Array|ContainsItem (Variables|/Script/Engine.Actor|GetTags OtherActor) "Belly")
    (if (Variables|Default|GetEntered)
      (Variables|Default|SetEntered false))))

(event EventBeginPlay)

(event Collision|EventActorBeginOverlap
  (params (OtherActor :type Actor%20Object%20Reference)))

(event EventTick
  (params (DeltaSeconds :type Float%20%28single-precision%29))
  (|CallParentFunction DeltaSeconds) ; This node is disabled and will not be called.\nDrag off pins to build functionality.
)

(fn ConstructionScript
  (|CallParentFunction))